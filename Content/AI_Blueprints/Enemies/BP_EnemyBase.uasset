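; BP_EnemyBase is an enemy character with sword combat, aggro state, health and spline patrolling, exposing actions and range getters.
; Montage-driven attack, wield and sheath events fire completion dispatchers; attacks damage the player by a simple distance check.
; Aggro swaps the mesh material, and patrol lookup steps along PatrolRoute spline points, reversing at the ends.
; Lethal point damage sets the blackboard Dead key, then ragdolls with a radial impulse before delayed destruction.
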(event Custom|Attack
  (bind _returnvalue (Game|GetPlayerCharacter 0))
  (Animation|Montage|PlayMontage (Variables|Character|GetMesh) "/Game/AI_Blueprints/Enemies/Animations/Sword_And_Shield_Slash_Anim1_Montage.Sword_And_Shield_Slash_Anim1_Montage"
    (:then
      (Audio|PlaySoundatLocation "/Game/Audio/Foley/Sword_Clash_Cue.Sword_Clash_Cue" (Transformation|GetActorLocation) "0, 0, 0" 1.0 1.0 0.0 0 0 0 0)
      (if (<= (Transformation|GetDistanceTo _returnvalue self) 2e+02)
        (bind _asbp_third_person_character (Utilities|Casting|CastToBP_ThirdPersonCharacter _returnvalue))
        (Default|TakeDamage _asbp_third_person_character)))
    (:OnCompleted
      (Default|CallAttackFinished :!label _label))
    (:OnInterrupted
      (goto _label))))

(event Custom|GetAggro
  (Rendering|Material|SetMaterial (Variables|Character|GetMesh) 0 "/Game/VFX/M5VFXVOL2/Materials/Etc/LightColor_Mat_Inst.LightColor_Mat_Inst")
  (Variables|Default|SetAggroed true))

(event Custom|LoseAggro
  (Rendering|Material|SetMaterial (Variables|Character|GetMesh) 0 (Variables|Default|GetOriginalMaterial))
  (Variables|Default|SetAggroed false))

(event Custom|Set%20Walk%20Speed
  (params (Speed :type Float%20%28double-precision%29))
  ;[0.06966 0.15 0.134] Sets max walk speed for BP_EnemyBase
  (Variables|/Script/Engine.CharacterMovementComponent|SetMaxWalkSpeed (Variables|Character|GetCharacterMovement) Speed))

(event Custom|Ragdoll
  (params (Origin :type Vector))
  (bind _mesh (Variables|Character|GetMesh))
  (AI|Components|Blackboard|SetValueasBool (AI|GetBlackboard 0) (Utilities|Name|MakeLiteralName "Dead") true)
  (Physics|SetSimulatePhysics _mesh true) ; Dont forget to change the collision presets to Ragdoll.
  (Physics|AddRadialForce _mesh (+ Origin "0.000000,0.000000,-100.000000") 5e+02 1e+05 "RIF_Linear" true)
  (Pawn|Components|CharacterMovement|DisableMovement (Variables|Character|GetCharacterMovement))
  (Collision|SetCollisionEnabled (Variables|Collision|GetCapsuleComponent) "NoCollision")
  (Utilities|FlowControl|Delay 5.0)
  (Actor|DestroyActor)
  (Actor|DestroyActor (Variables|Default|GetSwordActor01)))

(event Custom|WieldSword
  (Animation|Montage|PlayMontage (Variables|Character|GetMesh) "/Game/AI_Blueprints/Enemies/Animations/Montage_UnsheathSword.Montage_UnsheathSword"
    (:then
      (bind _returnvalue (Game|SpawnActorfromClass "/Game/Dark_Knight/Meshes/Weapons/BP_Sword01.BP_Sword01_C" (Transformation|GetActorTransform) "Undefined" "MultiplyWithRoot" 0 0))
      (bind _output_get (Variables|Default|SetSwordActor01 _returnvalue))
      (Transformation|AttachComponentToComponent _output_get (Variables|Character|GetMesh) "hand_r_Sword01_Socket" "SnapToTarget" "SnapToTarget" "SnapToTarget" true)
      (Variables|Default|SetIsWieldingSword true))
    (:OnCompleted
      (Default|CallOnWieldSword))))

(event Custom|SheathSword
  (Animation|Montage|PlayMontage (Variables|Character|GetMesh) "/Game/AI_Blueprints/Enemies/Animations/Montage_Sheath_sword.Montage_Sheath_sword"
    (:then
      (Actor|DestroyActor (Variables|Default|GetSwordActor))
      (Variables|Default|SetIsWieldingSword false))
    (:OnCompleted
      (Default|CallOnSheathSword))))

(event EventBeginPlay
  (Variables|Default|SetOriginalMaterial (Rendering|Material|GetMaterial (Variables|Character|GetMesh) 0)))

(event Game|Damage|EventPointDamage
  (params (Damage :type Float%20%28single-precision%29) (DamageType :type Damage%20Type%20Object%20Reference) (HitLocation :type Vector :default "0, 0, 0") (HitNormal :type Vector :default "0, 0, 0") (HitComponent :type Primitive%20Component%20Object%20Reference) (BoneName :type Name :default "None") (ShotFromDirection :type Vector :default "0, 0, 0") (InstigatedBy :type Controller%20Object%20Reference) (DamageCauser :type Actor%20Object%20Reference) (HitInfo :type Hit%20Result%20Structure%20%28by%20ref%29))
  (bind _output_get (Variables|Default|SetHealth (- (Variables|Default|GetHealth) Damage)))
  (if (<= _output_get 0.0)
    (CallFunction|Ragdoll HitLocation)))

(fn ConstructionScript)

(fn GetNextPatrolPointLocation
  (Utilities|IsValid (Variables|PatrolRoute|GetPatrolRoute)
    (:Is%20Valid
      (Variables|PatrolRoute|SetPatrol%20Point%20Index (+ (Variables|PatrolRoute|GetPatrol%20Point%20Index) (Variables|PatrolRoute|GetPatrolRouteDirection)))
      (if (or (>= (Variables|PatrolRoute|GetPatrol%20Point%20Index) (Spline|GetNumberOfSplinePoints (Variables|/Game/AI_Blueprints/Enemies/BP_PatrolRoute.BP_PatrolRoute_C|GetSpline (Variables|PatrolRoute|GetPatrolRoute)))) (<= (Variables|PatrolRoute|GetPatrol%20Point%20Index) 0))
        (Variables|PatrolRoute|SetPatrolRouteDirection (* (Variables|PatrolRoute|GetPatrolRouteDirection) -1)))
      (return "0, 0, 0" (Spline|GetLocationatSplinePoint (Variables|/Game/AI_Blueprints/Enemies/BP_PatrolRoute.BP_PatrolRoute_C|GetSpline (Variables|PatrolRoute|GetPatrolRoute)) (Variables|PatrolRoute|GetPatrol%20Point%20Index) "World")))))

(fn GetIdealRange
  (return (Variables|AICombat|GetAttack%20Radius) (Variables|AICombat|GetStrafe%20Radius)))

(fn PatrolRoute2
  (return (Variables|PatrolRoute|GetPatrolRoute2_0)))