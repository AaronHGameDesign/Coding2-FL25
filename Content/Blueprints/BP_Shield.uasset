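; BP_Shield is a shield item that can be picked up, used and dropped.
; Pickup disables collision and physics and snaps it to the hand_l socket, printing a message that names it "Machine Gun"; Drop detaches and restores both.
; Primary use only prints "Blocking".
; Secondary use flip-flops the shield between two relative positions, destroying BP_AiMoveTo actors overlapping its Box on every second use.
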(event EventPickup
  (params (SkeletalMesh :type Skeletal%20Mesh%20Component%20Object%20Reference))
  (bind _shield (Variables|Default|GetShield))
  ;[0.15 0.15 0.15 0.5] Pickup Function
  (Development|PrintText (Utilities|Text|FormatText "{name} is getting picked up and attached to {mesh}." (Utilities|String|MakeLiteralString "Machine Gun") SkeletalMesh) true true "(R=1.000000,G=0.174349,B=0.977565,A=1.000000)")
  (Collision|SetCollisionEnabled _shield "NoCollision")
  (Physics|SetSimulatePhysics _shield false)
  (Transformation|AttachComponentToComponent SkeletalMesh "hand_l" "SnapToTarget" "SnapToTarget" "KeepRelative" true))

(event EventUsePrimary
  (Development|PrintText "Blocking"))

(event EventDrop
  (bind _shield (Variables|Default|GetShield))
  (Transformation|DetachFromActor "KeepWorld" "KeepWorld" "KeepRelative")
  (Collision|SetCollisionEnabled _shield "QueryAndPhysics")
  (Physics|SetSimulatePhysics _shield true)
  (Utilities|FlowControl|Delay 0.2))

(event EventUseSecondary
  (bind _shield (Variables|Default|GetShield))
  (Development|PrintString "Secondary block")
  (Utilities|FlowControl|FlipFlop
    (:A
      (Transformation|SetRelativeLocation _shield "-10.000000,7.000000,0.000000" false false))
    (:B
      (Transformation|SetRelativeLocation _shield "0.000000,90.000000,0.000000" false false)
      (for _array_element (Collision|GetOverlappingActors (Variables|Default|GetBox) "/Game/AI_Blueprints/Enemies/BP_AiMoveTo.BP_AiMoveTo_C" :!class /Script/Engine.PrimitiveComponent)
        (Development|PrintString "killed the pest" true true "(R=1.000000,G=0.001747,B=0.000000,A=1.000000)")
        (Actor|DestroyActor _array_element)))))

(fn ConstructionScript)