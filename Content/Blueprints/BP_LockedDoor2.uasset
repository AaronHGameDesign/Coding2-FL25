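; BP_LockedDoor2 is a door the player opens and closes with the interact key while carrying a key.
; Its trigger caches the overlapping third-person character, enables input and opens a gate, reversing the latter two on exit.
; Interact checks the character's TotalKeys, playing either a locked sound or an opening sound.
; With keys, a gated FlipFlop plays or reverses a timeline that lerps door yaw between closed and open angles.
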(event OnComponentEndOverlap(Trigger)
  (params (OverlappedComponent :type Primitive%20Component%20Object%20Reference) (OtherActor :type Actor%20Object%20Reference) (OtherComp :type Primitive%20Component%20Object%20Reference) (OtherBodyIndex :type Integer))
  ;[1 0.8992 0.332] Open the door if player is close enough and has key.
  (Utilities|Casting|CastToBP_ThirdPersonCharacter OtherActor)
  (Input|DisableInput (Game|GetPlayerController 0))
  (Utilities|FlowControl|Gate true) ; enters at Close
)

(event OnComponentBeginOverlap(Trigger)
  (params (OverlappedComponent :type Primitive%20Component%20Object%20Reference) (OtherActor :type Actor%20Object%20Reference) (OtherComp :type Primitive%20Component%20Object%20Reference) (OtherBodyIndex :type Integer) (bFromSweep :type Boolean) (SweepResult :type Hit%20Result%20Structure%20%28by%20ref%29))
  ;[1 0.8992 0.332] Open the door if player is close enough and has key.
  (bind _asbp_third_person_character (Utilities|Casting|CastToBP_ThirdPersonCharacter OtherActor))
  (Input|EnableInput (Game|GetPlayerController 0))
  (Utilities|FlowControl|Gate true) ; enters at Open
)

(event EventBeginPlay
  ;[1 0.8992 0.332] Open the door if player is close enough and has key.
)

(event Input|ActionEvents|InputActioninteract
  (params (Key :type Key%20Structure :default "None"))
  ;[1 0.8992 0.332] Open the door if player is close enough and has key.
  (:Pressed
    (if (Variables|/Game/ThirdPerson/Blueprints/BP_ThirdPersonCharacter.BP_ThirdPersonCharacter_C|GetTotalKeys (stale OnComponentBeginOverlap(Trigger) _asbp_third_person_character))
      (Audio|PlaySoundatLocation "/Game/SFX/Door_Opening_Sound_Cue.Door_Opening_Sound_Cue" (Transformation|GetActorLocation) "0, 0, 0" 1.0 1.0 0.0 0 0 0 0)
      (Utilities|FlowControl|Gate true
        (:Exit
          ;[0.1929 1 0.2028] Open/Close Door Animation.
          (Utilities|FlowControl|FlipFlop
            (:A
              (bind _doortrack (Timeline|Open/CloseDoor Play)
                (:Update
                  (Transformation|SetRelativeRotation (Variables|Default|GetDoor) (Math|Rotator|MakeRotator 0.0 0.0 (Math|Float|Lerp (Variables|Default|GetClosedAngle) (Variables|Default|GetOpenAngle) _doortrack)) false false))))
            (:B
              (Timeline|Open/CloseDoor Reverse)))))
      (else
        (Audio|PlaySoundatLocation "/Game/SFX/LockedDoor_Cue.LockedDoor_Cue" (Transformation|GetActorLocation) "0, 0, 0" 1.0 1.0 0.0 0 0 0 0)))))

(fn ConstructionScript)