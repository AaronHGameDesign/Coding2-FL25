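; BP_ElementalBarrier is a barrier actor with an elemental type that ends the game when a player character without the matching immunity touches it.
; On BeginPlay it switches on ElementalType to set its TextRender, though every branch's text literal is empty here.
; Cube overlap casts to BP_ThirdPersonCharacter and compares ElementalImmunity with the barrier's type; a mismatch prints a message, waits briefly, then quits the game.
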(event OnComponentBeginOverlap(Cube)
  (params (OverlappedComponent :type Primitive%20Component%20Object%20Reference) (OtherActor :type Actor%20Object%20Reference) (OtherComp :type Primitive%20Component%20Object%20Reference) (OtherBodyIndex :type Integer) (bFromSweep :type Boolean) (SweepResult :type Hit%20Result%20Structure%20%28by%20ref%29))
  (bind _asbp_third_person_character (Utilities|Casting|CastToBP_ThirdPersonCharacter OtherActor))
  (if (not (Utilities|Enum|Equal(Enum) (Variables|Default|GetElementalType) (Variables|/Game/ThirdPerson/Blueprints/BP_ThirdPersonCharacter.BP_ThirdPersonCharacter_C|GetElementalImmunity _asbp_third_person_character)))
    (Development|PrintText "Hello")
    (Utilities|FlowControl|Delay 2.0)
    (Game|QuitGame 0 "Quit" false)))

(event EventBeginPlay
  (Development|PrintText "Hello")
  (switch Utilities|FlowControl|Switch|SwitchonElementalType (Variables|Default|GetElementalType)
    (:NewEnumerator1
      (Rendering|Components|TextRender|SetText (Variables|Default|GetTextRender) (Utilities|Text|MakeLiteralText "")))
    (:NewEnumerator2
      (Rendering|Components|TextRender|SetText (Variables|Default|GetTextRender) (Utilities|Text|MakeLiteralText "")))
    (:NewEnumerator3
      (Rendering|Components|TextRender|SetText (Variables|Default|GetTextRender) (Utilities|Text|MakeLiteralText "")))
    (:NewEnumerator4
      (Rendering|Components|TextRender|SetText (Variables|Default|GetTextRender) (Utilities|Text|MakeLiteralText "")))
    (:NewEnumerator5
      (Rendering|Components|TextRender|SetText (Variables|Default|GetTextRender) (Utilities|Text|MakeLiteralText "")))
    (:NewEnumerator6
      (Rendering|Components|TextRender|SetText (Variables|Default|GetTextRender) (Utilities|Text|MakeLiteralText "")))))

(fn ConstructionScript)