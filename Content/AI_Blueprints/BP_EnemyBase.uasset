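; Base enemy character that patrols, toggles aggro, attacks the player and dies into a ragdoll.
; Attack plays a wheel-kick montage and calls AttackFinished when it completes or is interrupted, while aggro changes swap the mesh material to red and back.
; Patrol lookup steps along a PatrolRoute spline, flipping direction at either end.
; Point damage reduces Health, and at zero triggers physics with a radial force from below the hit location.
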(event Custom|Attack
  (Development|PrintString "Attacking Player")
  (Animation|Montage|PlayMontage (Variables|Character|GetMesh) "/Game/CloseCombatAnimSet/Animations/InPlace/Attacks/NinjaWheelKick_Montage.NinjaWheelKick_Montage"
    (:OnCompleted
      _)
    (:OnInterrupted
      _))
  (Default|CallAttackFinished))

(event Custom|GetAggro
  (Rendering|Material|SetMaterial (Variables|Character|GetMesh) 0 "/AnimationSharing/AnimSharingRed.AnimSharingRed")
  (Variables|Default|SetAggroed true))

(event Custom|LoseAggro
  (Rendering|Material|SetMaterial (Variables|Character|GetMesh) 0 (Variables|Default|GetOriginalMaterial))
  (Variables|Default|SetAggroed false))

(event Custom|Set%20Walk%20Speed
  (params (Speed :type Float%20%28double-precision%29))
  ;[0.06966 0.15 0.134] Sets max walk speed for BP_EnemyBase
  (Variables|/Script/Engine.CharacterMovementComponent|SetMaxWalkSpeed (Variables|Character|GetCharacterMovement) Speed))

(event Custom|Ragdoll
  (params (Origin :type Vector))
  (bind _mesh (Variables|Character|GetMesh))
  (Physics|SetSimulatePhysics _mesh true) ; Dont forget to change the collision presets to Ragdoll.
  (Physics|AddRadialForce _mesh (+ Origin "0.000000,0.000000,-100.000000") 5e+02 1e+05 "RIF_Linear" true)
  (Pawn|Components|CharacterMovement|DisableMovement (Variables|Character|GetCharacterMovement)))

(event EventBeginPlay
  (Variables|Default|SetOriginalMaterial (Rendering|Material|GetMaterial (Variables|Character|GetMesh) 0)))

(event Game|Damage|EventAnyDamage
  (params (Damage :type Float%20%28single-precision%29) (DamageType :type Damage%20Type%20Object%20Reference) (InstigatedBy :type Controller%20Object%20Reference) (DamageCauser :type Actor%20Object%20Reference)))

(event Game|Damage|EventPointDamage
  (params (Damage :type Float%20%28single-precision%29) (DamageType :type Damage%20Type%20Object%20Reference) (HitLocation :type Vector :default "0, 0, 0") (HitNormal :type Vector :default "0, 0, 0") (HitComponent :type Primitive%20Component%20Object%20Reference) (BoneName :type Name :default "None") (ShotFromDirection :type Vector :default "0, 0, 0") (InstigatedBy :type Controller%20Object%20Reference) (DamageCauser :type Actor%20Object%20Reference) (HitInfo :type Hit%20Result%20Structure%20%28by%20ref%29))
  (Development|PrintText (Utilities|Text|FormatText "{instigator} damaged us for {dmg} damage!" InstigatedBy Damage) true true "(R=0.000000,G=0.660000,B=1.000000,A=1.000000)" 5.0)
  (bind _output_get (Variables|Default|SetHealth (- (Variables|Default|GetHealth) Damage)))
  (if (<= _output_get 0.0)
    (CallFunction|Ragdoll HitLocation)))

(fn ConstructionScript)

(fn GetNextPatrolPointLocation
  (Utilities|IsValid (Variables|PatrolRoute|GetPatrolRoute)
    (:Is%20Valid
      (Variables|PatrolRoute|SetPatrol%20Point%20Index (+ (Variables|PatrolRoute|GetPatrol%20Point%20Index) (Variables|PatrolRoute|GetPatrolRouteDirection)))
      (if (or (>= (Variables|PatrolRoute|GetPatrol%20Point%20Index) (Spline|GetNumberOfSplinePoints (Variables|/Game/AI_Blueprints/BP_PatrolRoute.BP_PatrolRoute_C|GetSpline (Variables|PatrolRoute|GetPatrolRoute)))) (<= (Variables|PatrolRoute|GetPatrol%20Point%20Index) 0))
        (Variables|PatrolRoute|SetPatrolRouteDirection (* (Variables|PatrolRoute|GetPatrolRouteDirection) -1)))
      (return "0, 0, 0" (Spline|GetLocationatSplinePoint (Variables|/Game/AI_Blueprints/BP_PatrolRoute.BP_PatrolRoute_C|GetSpline (Variables|PatrolRoute|GetPatrolRoute)) (Variables|PatrolRoute|GetPatrol%20Point%20Index) "World")))
    (:Is%20Not%20Valid
      (Development|PrintString "No patrol route end only"))))

(fn GetIdealRange
  (return (Variables|AICombat|GetAttack%20Radius) (Variables|AICombat|GetStrafe%20Radius)))