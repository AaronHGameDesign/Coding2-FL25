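; BP_MachineGun is a weapon that can be picked up, dropped and fired to launch projectiles.
; Pickup prints a debug message, turns off body physics and collision, snaps to the given skeletal mesh's hand_r socket, then adjusts scale and offset.
; Drop detaches it, restores physics and collision, and rescales the body.
; UsePrimary spawns a BP_Projectile at the Barrel and propels its sphere with a force along the body's forward vector.
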(event EventUsePrimary
  (bind _barrel (Variables|Default|GetBarrel))
  (bind _returnvalue (Transformation|GetWorldTransform _barrel))
  (bind _returnvalue_2 (Game|SpawnActorfromClass "/Game/Blueprints/BP_Projectile.BP_Projectile_C" (Math|Transform|MakeTransform (.location _returnvalue) (.rotation _returnvalue) (.scale _returnvalue)) "AlwaysSpawn" "MultiplyWithRoot" 0 0))
  (Physics|AddForce (Variables|/Game/Blueprints/BP_Projectile.BP_Projectile_C|GetSphere _returnvalue_2) (* (Math|Vector|GetForwardVector (Variables|Default|GetMachineGunBody)) 5e+05) "None" true))

(event EventDrop
  (bind _machinegunbody (Variables|Default|GetMachineGunBody))
  (Transformation|DetachFromActor "KeepWorld" "KeepWorld" "KeepRelative")
  (Collision|SetCollisionEnabled _machinegunbody "QueryAndPhysics")
  (Physics|SetSimulatePhysics _machinegunbody true)
  (Transformation|SetRelativeScale3D _machinegunbody "2.000000,0.500000,0.400000"))

(event EventPickup
  (params (SkeletalMesh :type Skeletal%20Mesh%20Component%20Object%20Reference))
  (bind _machinegunbody (Variables|Default|GetMachineGunBody))
  (bind _machinegunbody_2 (Variables|Default|GetMachineGunBody))
  ;[0.15 0.15 0.15 0.5] Pickup Function
  (Development|PrintText (Utilities|Text|FormatText "{name} is getting picked up and attached to {mesh}." (Utilities|String|MakeLiteralString "Machine Gun") SkeletalMesh) true true "(R=1.000000,G=0.174349,B=0.977565,A=1.000000)")
  (Physics|SetSimulatePhysics _machinegunbody_2 false)
  (Collision|SetCollisionEnabled _machinegunbody_2 "NoCollision")
  (Transformation|AttachComponentToComponent SkeletalMesh "hand_r" "SnapToTarget" "SnapToTarget" "KeepRelative" true)
  (Transformation|SetRelativeScale3D _machinegunbody "0.200000,0.250000,1.000000")
  (Transformation|SetRelativeLocation _machinegunbody "-10.000000,0.000000,40.000000" false false))

(fn ConstructionScript)