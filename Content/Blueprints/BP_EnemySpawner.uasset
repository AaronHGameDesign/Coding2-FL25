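; Enemy spawner that populates the level with randomized AI enemies at BeginPlay.
; It visits every BP_EnemySpawnPoint and, with a weighted chance, spawns a BP_AiMoveTo at that point's transform.
; Each spawned enemy gets a random skeletal mesh, name and material from the spawner's arrays.
; A final pass writes the Name of every BP_AiMoveTo in the level into its name text.
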(event EventBeginPlay
  (bind _outactors (Actor|GetAllActorsOfClass "/Game/Blueprints/BP_EnemySpawnPoint.BP_EnemySpawnPoint_C"))
  (for _array_element _outactors
    (if (Math|Random|RandomBoolwithWeight 0.75)
      (bind _returnvalue (Game|SpawnActorfromClass "/Game/AI_Blueprints/Enemies/BP_AiMoveTo.BP_AiMoveTo_C" (Transformation|GetActorTransform _array_element) "Undefined" "MultiplyWithRoot" _array_element 0))
      (if (Utilities|IsValid _returnvalue)
        (Components|SkeletalMesh|SetSkeletalMeshAsset (Variables|/Script/Engine.Character|GetMesh _returnvalue) (.OutItem (Utilities|Array|Random (Variables|Default|GetMeshes))))
        (Variables|/Game/AI_Blueprints/Enemies/BP_AiMoveTo.BP_AiMoveTo_C|SetName _returnvalue (.OutItem (Utilities|Array|Random (Variables|Default|GetEnemyNamesArray))))
        (Rendering|Material|SetMaterial (Variables|/Script/Engine.Character|GetMesh _returnvalue) 0 (.OutItem (Utilities|Array|Random (Variables|Default|GetMaterial)))))))
  (bind _outactors_2 (Actor|GetAllActorsOfClass "/Game/AI_Blueprints/Enemies/BP_AiMoveTo.BP_AiMoveTo_C"))
  (for _array_element_2 _outactors_2
    (Rendering|Components|TextRender|SetText (Variables|/Game/AI_Blueprints/Enemies/BP_AiMoveTo.BP_AiMoveTo_C|GetAi%20Name%20Text _array_element_2) (Utilities|Text|ToText(Name) (Variables|/Game/AI_Blueprints/Enemies/BP_AiMoveTo.BP_AiMoveTo_C|GetName _array_element_2)))))

(fn ConstructionScript)