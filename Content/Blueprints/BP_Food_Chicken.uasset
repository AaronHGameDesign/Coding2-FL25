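; BP_Food_Chicken is a holdable chicken food item that the third-person character picks up by overlapping its trigger.
; Pickup attaches the chicken mesh to a right-hand socket without collision.
; Drop detaches it and enables physics and collision, restoring its saved world location so it falls in place.
; UsePrimary is empty; the placeholder health message, item destruction and sound playback are unconnected.
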(event OnComponentBeginOverlap(PickupTrigger)
  (params (OverlappedComponent :type Primitive%20Component%20Object%20Reference) (OtherActor :type Actor%20Object%20Reference) (OtherComp :type Primitive%20Component%20Object%20Reference) (OtherBodyIndex :type Integer) (bFromSweep :type Boolean) (SweepResult :type Hit%20Result%20Structure%20%28by%20ref%29))
  (bind _asbp_third_person_character (Utilities|Casting|CastToBP_ThirdPersonCharacter OtherActor))
  (Default|Pickup self 0 _asbp_third_person_character))

(event EventPickup
  (params (SkeletalMesh :type Skeletal%20Mesh%20Component%20Object%20Reference) (PlayerRef :type BP%20Third%20Person%20Character%20Object%20Reference))
  (Transformation|AttachComponentToComponent (Variables|Default|GetChicken) SkeletalMesh "hand_r_Sword_Socket" "SnapToTarget" "KeepRelative" "KeepRelative" true)
  (Collision|SetCollisionEnabled (Variables|Default|GetChicken) "NoCollision") ; Collide with the ground please
)

(event EventDrop
  (bind _chicken (Variables|Default|GetChicken))
  (Variables|Default|SetDropLocation (Transformation|GetWorldLocation _chicken))
  (Transformation|DetachFromComponent _chicken "KeepRelative" "KeepRelative" "KeepRelative" true) ; Don't follow the hand anymore
  (Physics|SetSimulatePhysics (Variables|Default|GetChicken) true) ; use gravity to fall
  (Collision|SetCollisionEnabled (Variables|Default|GetChicken) "QueryAndPhysics") ; Collide with the ground please
  (Transformation|SetWorldLocation (Variables|Default|GetChicken) (Variables|Default|GetDropLocation) false false) ; To prevent the can from going to world origin
)

(event EventUsePrimary
  ;[1 1 1] Comment
)

(fn ConstructionScript)