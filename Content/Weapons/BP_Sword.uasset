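; BP_Sword is a sword weapon that a player can pick up, wield and drop.
; Pickup stores the player, sets its IsWieldSword flag, prints a debug message, disables mesh collision and physics, then snaps to the hand socket of the passed skeletal mesh.
; Drop clears the flag, detaches while keeping world location and rotation, and restores collision and physics on the mesh.
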(event EventPickup
  (params (SkeletalMesh :type Skeletal%20Mesh%20Component%20Object%20Reference) (PlayerRef :type BP%20Third%20Person%20Character%20Object%20Reference))
  (bind _swordmesh (Variables|Default|GetSwordMesh))
  ;[0.15 0.15 0.15 0.5] Pickup Function
  (bind _output_get (Variables|Default|SetPlayer%20Ref PlayerRef))
  (Variables|/Game/ThirdPerson/Blueprints/BP_ThirdPersonCharacter.BP_ThirdPersonCharacter_C|SetIsWieldSword? _output_get true)
  (Development|PrintText (Utilities|Text|FormatText "{name} is getting picked up and attached to {mesh}." (Utilities|String|MakeLiteralString "Sword") SkeletalMesh) true true "(R=1.000000,G=0.174349,B=0.977565,A=1.000000)")
  (Collision|SetCollisionEnabled _swordmesh "NoCollision")
  (Physics|SetSimulatePhysics _swordmesh false)
  (Transformation|AttachComponentToComponent SkeletalMesh "hand_r_Sword_Socket" "SnapToTarget" "SnapToTarget" "SnapToTarget" true))

(event EventDrop
  (bind _swordmesh (Variables|Default|GetSwordMesh))
  (Variables|/Game/ThirdPerson/Blueprints/BP_ThirdPersonCharacter.BP_ThirdPersonCharacter_C|SetIsWieldSword? (Variables|Default|GetPlayer%20Ref) false)
  (Transformation|DetachFromActor "KeepWorld" "KeepWorld" "KeepRelative")
  (Collision|SetCollisionEnabled _swordmesh "QueryAndPhysics")
  (Physics|SetSimulatePhysics _swordmesh true))

(fn ConstructionScript)