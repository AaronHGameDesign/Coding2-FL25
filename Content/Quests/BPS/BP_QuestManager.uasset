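; Quest manager that starts quests from DT_Quests, including auto-start rows, and tracks active, completed and per-quest progress.
; Starting blocks active or completed non-repeatable quests.
; Completing an objective rewrites nested structs and checks for quest completion, though it matches ObjectiveID against QuestID and lookups stop at the first active quest.
; Finished quests show WBP_StartedQuest, move to CompletedQuests and drop their progress.
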(event EventQMCompleteObjective
  (params (QuestID :type Name :default "None") (ObjectiveID :type Name :default "None"))
  (bind _output (CallFunction|CompleteObjective QuestID ObjectiveID))
  (if _output
    (CallFunction|CompleteQuest QuestID)))

(event EventQMAutoStartQuests
  (bind _outrownames (DataTable|GetDataTableRowNames "/Game/Quests/DataTables/DT_Quests.DT_Quests"))
  (for _array_element _outrownames
    (bind _returnvalue (Utilities|GetDataTableRow "/Game/Quests/DataTables/DT_Quests.DT_Quests" _array_element)
      (:then
        (if (.AutoStart (Utilities|Struct|BreakS_QuestData _returnvalue))
          (CallFunction|StartQuest (.QuestID (Utilities|Struct|BreakS_QuestData _returnvalue))))))))

(event EventQMStartQuest
  (params (QuestID :type Name :default "None"))
  (CallFunction|StartQuest QuestID))

(fn ConstructionScript)

(fn StartQuest
  (params (QuestID :type Name))
  (bind _canstart_ (CallFunction|CheckifQuestHasAlreadyBeenStarted QuestID))
  (if _canstart_
    (bind _returnvalue (Utilities|GetDataTableRow "/Game/Quests/DataTables/DT_Quests.DT_Quests" QuestID)
      (:then
        (Utilities|Array|Add (Variables|Default|GetActiveQuests) _returnvalue)
        (LocalVariables|SetTempProgress (Variables|Default|GetQuestProgress))
        (Utilities|Map|Add (LocalVariables|GetTempProgress) QuestID 0)
        (Variables|Default|SetQuestProgress (LocalVariables|GetTempProgress))))))

(fn CompleteObjective
  (params (QuestID :type Name) (ObjectiveID :type Name))
  (bind _completed_ (CallFunction|UpdateObjectiveCompletion QuestID ObjectiveID))
  (LocalVariables|SetTempProgress (Variables|Default|GetQuestProgress))
  (if (.ReturnValue (Utilities|Map|Find (LocalVariables|GetTempProgress) QuestID))
    (bind _result (Math|Integer|IncrementInt (.Value (Utilities|Map|Find (LocalVariables|GetTempProgress) QuestID)))
      (:%20%20
        (Utilities|Map|Add (LocalVariables|GetTempProgress) QuestID _result)
        (Variables|Default|SetQuestProgress (LocalVariables|GetTempProgress))
        (bind _returnvalue (Utilities|GetDataTableRow "/Game/Quests/DataTables/DT_Quests.DT_Quests" QuestID)
          (:then
            (for _array_element (.Objectives (Utilities|Struct|BreakS_QuestData _returnvalue))
              (if (== (.ObjectiveID (Utilities|Struct|BreakS_QuestObjectives _array_element)) ObjectiveID)
                _))
            (return _completed_)))))
    (else
      (return false))))

(fn UpdateObjectiveCompletion
  (params (QuestID :type Name) (ObjectiveID :type Name))
  (for (_array_element _array_index) (Variables|Default|GetActiveQuests)
    (LocalVariables|SetTempObjectives (.Objectives (Utilities|Struct|BreakS_QuestData _array_element)))
    (if (== (.QuestID (Utilities|Struct|BreakS_QuestData _array_element)) QuestID)
      (for (_array_element_2 _array_index_2) (.Objectives (Utilities|Struct|BreakS_QuestData _array_element))
        (if (== (.ObjectiveID (Utilities|Struct|BreakS_QuestObjectives _array_element_2)) QuestID)
          (Utilities|Array|SetArrayElem (LocalVariables|GetTempObjectives) _array_index_2 (Utilities|Struct|MakeS_QuestObjectives (.ObjectiveID (Utilities|Struct|BreakS_QuestObjectives _array_element_2)) (.Description (Utilities|Struct|BreakS_QuestObjectives _array_element_2)) true (.ObjectiveType (Utilities|Struct|BreakS_QuestObjectives _array_element_2)) (.TargetData (Utilities|Struct|BreakS_QuestObjectives _array_element_2)) (.Optional (Utilities|Struct|BreakS_QuestObjectives _array_element_2)) (.CanCompleteAnOrder? (Utilities|Struct|BreakS_QuestObjectives _array_element_2))))
          (Utilities|Array|SetArrayElem (Variables|Default|GetActiveQuests) _array_index (Utilities|Struct|MakeS_QuestData (.QuestID (Utilities|Struct|BreakS_QuestData _array_element)) (.Title (Utilities|Struct|BreakS_QuestData _array_element)) (.Description (Utilities|Struct|BreakS_QuestData _array_element)) (LocalVariables|GetTempObjectives) (.IsRepeatable (Utilities|Struct|BreakS_QuestData _array_element)) (.AutoStart (Utilities|Struct|BreakS_QuestData _array_element)) (.Rewards (Utilities|Struct|BreakS_QuestData _array_element))))
          (bind _completed_ (CallFunction|CheckQuestCompleted (.QuestID (Utilities|Struct|BreakS_QuestData _array_element))))
          (return _completed_)))
      (else
        (return false)))))

(fn CheckQuestCompleted
  (params (QuestID :type Name))
  (for _array_element (Variables|Default|GetActiveQuests)
    (if (== (.QuestID (Utilities|Struct|BreakS_QuestData _array_element)) QuestID)
      (for _array_element_2 (.Objectives (Utilities|Struct|BreakS_QuestData _array_element))
        (if (not (.IsCompleted (Utilities|Struct|BreakS_QuestObjectives _array_element_2)))
          (return false)))
      (return true)
      (else
        (return false)))))

(fn CompleteQuest
  (params (QuestID :type Name))
  (for _array_element (Variables|Default|GetActiveQuests)
    (if (== (.QuestID (Utilities|Struct|BreakS_QuestData _array_element)) QuestID)
      (bind _returnvalue (UserInterface|CreateWidget "/Game/Quests/Widgets/WBP_StartedQuest.WBP_StartedQuest_C" 0 _array_element))
      (UserInterface|Viewport|AddtoViewport _returnvalue 0)
      (Utilities|Array|Add (Variables|Default|GetCompletedQuests) _array_element)
      (Utilities|Array|RemoveItem (Variables|Default|GetActiveQuests) _array_element)
      (Utilities|Map|Remove (Variables|Default|GetQuestProgress) QuestID)
      (return))))

(fn CheckifQuestHasAlreadyBeenStarted
  (params (QuestID :type Name))
  (for _array_element (Variables|Default|GetCompletedQuests)
    (if (and (== (.QuestID (Utilities|Struct|BreakS_QuestData _array_element)) QuestID) (not (.IsRepeatable (Utilities|Struct|BreakS_QuestData _array_element))))
      (return false)))
  (for _array_element_2 (Variables|Default|GetActiveQuests)
    (if (== (.QuestID (Utilities|Struct|BreakS_QuestData _array_element_2)) QuestID)
      (return false)))
  (return true))