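; BP_LoopsandLists is a demonstration Blueprint for loops and arrays, with results printed as debug text.
; BeginPlay finds every BP_AiMoveTo actor and prints its name.
; DelayLoop repeats endlessly through a short Delay and self-call, counting passes and calling PrintColors, which shuffles TextColors and prints a randomly colored line per element.
; The startup call to DelayLoop is disconnected, so only the actor listing runs on BeginPlay.
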(event Custom|Delay%20Loop
  (Development|PrintString (Utilities|String|Append "Starting Delay Loop #" (Utilities|String|ToString(Integer) (Variables|Default|GetDelayLoopCounter))))
  (Math|Integer|IncrementInt (Variables|Default|GetDelayLoopCounter)
    (:%20%20
      (Utilities|FlowControl|Delay 0.1)
      (CallFunction|PrintColors)
      (CallFunction|DelayLoop))))

(event Custom|Print%20Colors
  (bind _array (Utilities|Array|MakeArray "(R=1.000000,G=0.243920,B=0.194149,A=1.000000)" "(R=0.180032,G=1.000000,B=0.239289,A=1.000000)" "(R=0.274162,G=0.359657,B=1.000000,A=1.000000)" "(R=1.000000,G=0.992662,B=0.288268,A=1.000000)"))
  (bind _textcolors (Variables|Default|GetTextColors))
  (bind (_outitem _outindex) (Utilities|Array|Random _array))
  (Utilities|Array|Shuffle _textcolors)
  (for _array_element _textcolors
    (Development|PrintString (Utilities|String|Append "Printing colored # " (Utilities|String|ToString(Integer) _outindex)) true true _outitem))
  (Development|PrintString "We are done printing colors"))

(event EventBeginPlay
  (bind _outactors (Actor|GetAllActorsOfClass "/Game/AI_Blueprints/Enemies/BP_AiMoveTo.BP_AiMoveTo_C"))
  (for _array_element _outactors
    (Development|PrintString (Utilities|String|ToString(Name) (Variables|/Game/AI_Blueprints/Enemies/BP_AiMoveTo.BP_AiMoveTo_C|GetName _array_element)))))

(fn ConstructionScript)